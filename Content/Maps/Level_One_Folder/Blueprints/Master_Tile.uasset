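; Master_Tile is a floor tile for an endless-runner level that chains new tiles as the player advances.
; The construction script gathers left, middle and right spawn points, then randomly adds either a blocker child actor at one of them or a few coins at random points inside CoinArea.
; When the ThirdPersonCharacter overlaps EndTrigger, it asks RunPersonGameMode to add a floor tile, then destroys itself after DestoryTime.
; GetAttachTranform exposes the AttachPoint world transform.
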(event `self.EndTrigger.OnComponentBeginOverlap`
  (params (OverlappedComponent :type "PrimitiveComponent Object Reference") (OtherActor :type "Actor Object Reference") (OtherComp :type "PrimitiveComponent Object Reference") (OtherBodyIndex :type Integer) (bFromSweep :type Boolean) (SweepResult :type "HitResult Structure (by ref)"))
  ;[0 1 1] ZP, Spawn and Destory Tiles
  (cast `/Game/ThirdPersonBP/Blueprints/ThirdPersonCharacter` OtherActor)
  (bind _asrun_person_game_mode (cast `/Game/Maps/Level_One_Folder/Blueprints/RunPersonGameMode` (`GameplayStatics.GetGameMode`)))
  (`/Game/Maps/Level_One_Folder/Blueprints/RunPersonGameMode.AddFloorTile` _asrun_person_game_mode)
  (`KismetSystemLibrary.Delay` (`self.Destory Time`))
  (`self.K2_DestroyActor`))

(fn `GetAttachTranform`
  (returns (AttachTransform :type "Transform Structure"))
  ;[0 1 1] ZP, Findding Attach Point
  (return (`SceneComponent.K2_GetComponentToWorld` (`self.AttachPoint`))))

(fn `SetSpawnPoints`
  (locals (NewLocalVar_0 :type "Transform Structure"))
  ;[0 1 1] ZP, Find Spawn Points
  (set `self.Spawn Points` (`|MakeArray` (`SceneComponent.GetRelativeTransform` (`self.Spawnpoint L`)) (`SceneComponent.GetRelativeTransform` (`self.Spawnpoint M`)) (`SceneComponent.GetRelativeTransform` (`self.Spawnpoint R`)))))

(fn `SpawnBlocker`
  (locals (NewLocalVar_0 :type "Transform Structure"))
  (bind _spawn_points (`self.Spawn Points`))
  ;[0 1 1] ZP, Spawning in Blocker
  (`AddComponent|NODE_AddChildActorComponent-0` :`RelativeTransform` (`|GetArrayItem` _spawn_points (`KismetMathLibrary.RandomIntegerInRange` 0 (`KismetArrayLibrary.Array_LastIndex` _spawn_points)))))

(fn `SpawnCoins`
  (bind _coin_area (`self.Coin Area`))
  ;[0 1 1] ZP, Spawns Coins
  (for _ (range (+ (`KismetMathLibrary.RandomIntegerInRange` 1 4) 1))
    (`AddComponent|NODE_AddChildActorComponent-1` :`RelativeTransform` (`KismetMathLibrary.Conv_VectorToTransform` (`KismetMathLibrary.RandomPointInBoundingBox` (`SceneComponent.RelativeLocation` _coin_area) (`BoxComponent.BoxExtent` _coin_area))))))

(fn `UserConstructionScript`
  ;[0 1 1] ZP, Set and Spawn Blocker
  (`self.SetSpawnPoints`)
  (switch `int` (`KismetMathLibrary.RandomIntegerInRange` 0 1)
    (:`Default`
      (`self.SpawnBlocker` :!label _label))
    (:`0`
      (`self.SpawnCoins`))
    (:`1`
      (goto _label))))